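; BP_ClimbingRoot is a climbable actor that carries the player along a spline in the vertical platformer.
; Overlapping its trigger box toggles the player's CanClimb flag, and a Climb event starts the movement.
; While climbing, Tick disables player input and collision and teleports the player along the spline at Speed.
; At the last point, input returns and EndClimb repositions the actor and trigger, restores collision and resets climb state.
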(event `self.ReceiveBeginPlay`
  (bind _returnvalue (`GameplayStatics.GetActorOfClass` "/Game/VerticalPlatformer/Blueprints/Player/BP_Player.BP_Player_C"))
  (set `self.PlayerRef` _returnvalue)
  (`ActorComponent.SetIsReplicated` (`self.SplineTrack`) false))

(event `self.BoxTriggerTop.OnComponentBeginOverlap`
  (params (OverlappedComponent :type "PrimitiveComponent Object Reference") (OtherActor :type "Actor Object Reference") (OtherComp :type "PrimitiveComponent Object Reference") (OtherBodyIndex :type Integer) (bFromSweep :type Boolean) (SweepResult :type "HitResult Structure (by ref)"))
  (if (== OtherActor (`self.PlayerRef`))
    (set `/Game/VerticalPlatformer/Blueprints/Player/BP_Player.CanClimb` true (`self.PlayerRef`))))

(event `self.BoxTriggerTop.OnComponentEndOverlap`
  (params (OverlappedComponent :type "PrimitiveComponent Object Reference") (OtherActor :type "Actor Object Reference") (OtherComp :type "PrimitiveComponent Object Reference") (OtherBodyIndex :type Integer))
  (if (== OtherActor (`self.PlayerRef`))
    (set `/Game/VerticalPlatformer/Blueprints/Player/BP_Player.CanClimb` false (`self.PlayerRef`))))

(event `Climb`
  (set `self.PlayerIsClimbingMe` true))

(event `self.ReceiveTick`
  (params (DeltaSeconds :type "Float (single-precision)"))
  (bind _splinetrack (`self.SplineTrack`))
  (bind _returnvalue_location (`KismetMathLibrary.BreakTransform` (`SplineComponent.GetTransformAtDistanceAlongSpline` (`self.SplineTrack`) (`self.Distance`) "World" false)))
  (if (`self.PlayerIsClimbingMe`)
    (`self.DisableInput` (`self.PlayerRef`) null)
    (set `self.Distance` (+ (* DeltaSeconds (`self.Speed`)) (`self.Distance`)))
    (`self.SetActorEnableCollision` (`self.PlayerRef`) false)
    (`self.K2_SetActorTransform` (`self.PlayerRef`) (`KismetMathLibrary.MakeTransform` _returnvalue_location) false true)
    (if (>= (`self.Distance`) (`SplineComponent.GetDistanceAlongSplineAtSplinePoint` _splinetrack (- (`SplineComponent.GetNumberOfSplinePoints` _splinetrack) 1)))
      (`self.EnableInput` (`self.PlayerRef`) null)
      (`self.EndClimb`))))

(fn `EndClimb`
  (bind _playerref (`self.PlayerRef`))
  (bind (_returnvalue_x _returnvalue_y _returnvalue_z) (`KismetMathLibrary.BreakVector` (`self.K2_GetActorLocation` (`self.PlayerRef`))))
  (`self.K2_SetActorLocation` (`KismetMathLibrary.MakeVector` _returnvalue_x _returnvalue_y (- _returnvalue_z 0.1)))
  (set `/Game/VerticalPlatformer/Blueprints/Player/BP_Player.isClimbing` false _playerref)
  (set `/Game/VerticalPlatformer/Blueprints/Player/BP_Player.CanClimb` false _playerref)
  (`SceneComponent.K2_SetRelativeLocation` (`self.BoxTriggerTop`) (`SplineComponent.GetLocationAtSplinePoint` (`self.SplineTrack`) 0 "World") false false)
  (`self.SetActorEnableCollision` (`self.PlayerRef`) true)
  (set `self.Distance` 0.0)
  (set `self.PlayerIsClimbingMe` false))

(fn `UserConstructionScript`)