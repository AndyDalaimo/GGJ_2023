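; Player Blueprint for a vertical platformer, handling movement along the world Y axis, jumping and the start of root climbing.
; BeginPlay caches a BP_ClimbingRoot reference, and the ClimbRoot input sets IsClimbing and prints a debug message when CanClimb is true.
; Climbing motion is unfinished: logic to advance a distance and snap the player to the root's spline transform is disconnected, and Tick does nothing.
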(event `self.ReceiveBeginPlay`
  (bind _returnvalue (`GameplayStatics.GetActorOfClass` "/Game/VerticalPlatformer/Blueprints/Platforming/BP_ClimbingRoot.BP_ClimbingRoot_C"))
  (set `self.ClimbingRootRef` _returnvalue))

(event `InputAxis|MoveRight`
  (params (AxisValue :type "Float (single-precision)"))
  ;[1 1 1] Player Movement
  (`self.AddMovementInput` (`KismetMathLibrary.MakeVector` 0.0 AxisValue) 0.2))

(event `InputAction|Jump`
  (params (Key :type "Key Structure"))
  ;[1 1 1] Player Movement
  (:`Pressed`
    (`self.Jump`))
  (:`Released`
    (`self.StopJumping`)))

(event `InputAxis|MoveLeft`
  (params (AxisValue :type "Float (single-precision)"))
  ;[1 1 1] Player Movement
  (`self.AddMovementInput` (`KismetMathLibrary.MakeVector` 0.0 AxisValue) 0.2))

(event `InputAction|ClimbRoot`
  (params (Key :type "Key Structure"))
  ;[1 1 1] Player Climbing
  (:`Pressed`
    (if (`self.CanClimb`)
      (`KismetSystemLibrary.PrintString` "Player Climbing")
      (set `self.isClimbing` true))))

(event `self.ReceiveTick`
  (params (DeltaSeconds :type "Float (single-precision)"))
  ;[1 1 1] Player Climbing
)

(fn `UserConstructionScript`)