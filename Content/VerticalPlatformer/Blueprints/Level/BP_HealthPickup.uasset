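; BP_HealthPickup is a level pickup that restores one point of health to the player.
; On BeginPlay it finds and caches the BP_Player instance with GetActorOfClass.
; When that player overlaps its Box with Health below a hardcoded cap of three, it increments Health, prints the new value and destroys itself.
; At full health, the pickup stays in place.
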(event `self.ReceiveBeginPlay`
  (bind _returnvalue (`GameplayStatics.GetActorOfClass` "/Game/VerticalPlatformer/Blueprints/Player/BP_Player.BP_Player_C"))
  (set `self.PlayerRef` _returnvalue))

(event `self.ReceiveTick`
  (params (DeltaSeconds :type "Float (single-precision)")))

(event `self.Box.OnComponentBeginOverlap`
  (params (OverlappedComponent :type "PrimitiveComponent Object Reference") (OtherActor :type "Actor Object Reference") (OtherComp :type "PrimitiveComponent Object Reference") (OtherBodyIndex :type Integer) (bFromSweep :type Boolean) (SweepResult :type "HitResult Structure (by ref)"))
  (bind _playerref (`self.PlayerRef`))
  (if (and (== OtherActor _playerref) (< (`/Game/VerticalPlatformer/Blueprints/Player/BP_Player.Health` _playerref) 3))
    (bind _result (`/Engine/EditorBlueprintResources/StandardMacros.IncrementInt` (`/Game/VerticalPlatformer/Blueprints/Player/BP_Player.Health` (`self.PlayerRef`)))
      (:`  `
        (`KismetSystemLibrary.PrintString` (`KismetStringLibrary.Concat_StrStr` "Player health: " (`KismetStringLibrary.Conv_IntToString` _result)))
        (`self.K2_DestroyActor`)))))

(fn `UserConstructionScript`)