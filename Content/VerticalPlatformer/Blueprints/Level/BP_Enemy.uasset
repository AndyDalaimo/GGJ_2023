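; BP_Enemy is a bug enemy that travels along a spline and damages the player on contact.
; Tick advances a distance by speed, places the bug at that point on the spline and wraps back to the start at the end.
; Capsule overlap with BP_Player plays sounds, decrements Health, copies it to a WBP_HUD instance created at BeginPlay, and calls OnDeath when health runs out.
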(event `self.ReceiveBeginPlay`
  (bind _returnvalue (`GameplayStatics.GetActorOfClass` "/Game/VerticalPlatformer/Blueprints/Player/BP_Player.BP_Player_C"))
  (set `self.PlayerRef` _returnvalue)
  (bind _returnvalue_2 (`|CreateWidget` "/Game/VerticalPlatformer/Blueprints/UI/WBP_HUD.WBP_HUD_C"))
  (set `self.HUDRef` _returnvalue_2))

(event `self.ReceiveTick`
  (params (DeltaSeconds :type "Float (single-precision)"))
  (bind _output_get (set `self.Distance` (+ (* DeltaSeconds (`self.Speed`)) (`self.Distance`))))
  (bind (_returnvalue_location _returnvalue_rotation) (`KismetMathLibrary.BreakTransform` (`SplineComponent.GetTransformAtDistanceAlongSpline` (`self.Spline`) _output_get "World" false)))
  (`SceneComponent.K2_SetWorldTransform` (`self.Bug`) (`KismetMathLibrary.MakeTransform` _returnvalue_location _returnvalue_rotation) false false)
  (if (>= (`self.Distance`) (`SplineComponent.GetSplineLength` (`self.Spline`)))
    (set `self.Distance` 0.0)))

(event `self.Capsule.OnComponentBeginOverlap`
  (params (OverlappedComponent :type "PrimitiveComponent Object Reference") (OtherActor :type "Actor Object Reference") (OtherComp :type "PrimitiveComponent Object Reference") (OtherBodyIndex :type Integer) (bFromSweep :type Boolean) (SweepResult :type "HitResult Structure (by ref)"))
  (bind _playerref (`self.PlayerRef`))
  (if (== OtherActor (`self.PlayerRef`))
    (`GameplayStatics.PlaySoundAtLocation` "/Game/VerticalPlatformer/Assets/Audio/InsectWings.InsectWings" (`self.K2_GetActorLocation`) (struct) 1.0 1.0 0.0 null null null null)
    (bind _result (`/Engine/EditorBlueprintResources/StandardMacros.DecrementInt` (`/Game/VerticalPlatformer/Blueprints/Player/BP_Player.Health` (`self.PlayerRef`)))
      (:`  `
        (set `/Game/VerticalPlatformer/Blueprints/UI/WBP_HUD.Health` _result (`self.HUDRef`))
        (`GameplayStatics.PlaySoundAtLocation` "/Game/VerticalPlatformer/Assets/Audio/BunnyHurt.BunnyHurt" (`self.K2_GetActorLocation` (`self.PlayerRef`)) (struct) 1.0 1.0 0.0 null null null null)
        (if (<= (`/Game/VerticalPlatformer/Blueprints/Player/BP_Player.Health` (`self.PlayerRef`)) 0)
          (set `/Game/VerticalPlatformer/Blueprints/Player/BP_Player.PlayCutscene` false _playerref)
          (`/Game/VerticalPlatformer/Blueprints/Player/BP_Player.OnDeath` _playerref))))))

(fn `UserConstructionScript`)