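; BP_StartingFlower is a flower actor in the vertical platformer's cinematics that dies when the smog reaches it.
; On BeginPlay it caches the BP_LevelPanner actor as the smog and the BP_StartingChar as the player.
; When the smog overlaps its Box, it marks itself dead, calls OnFlowerDied on the character and sets its paper flipbook to FB_Flower.
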(event `self.ReceiveBeginPlay`
  (bind _returnvalue (`GameplayStatics.GetActorOfClass` "/Game/VerticalPlatformer/Blueprints/Level/BP_LevelPanner.BP_LevelPanner_C"))
  (set `self.SmogRef` _returnvalue)
  (bind _returnvalue_2 (`GameplayStatics.GetActorOfClass` "/Game/VerticalPlatformer/Cinematics/BP_StartingChar.BP_StartingChar_C"))
  (set `self.PlayerRef` _returnvalue_2))

(event `self.Box.OnComponentBeginOverlap`
  (params (OverlappedComponent :type "PrimitiveComponent Object Reference") (OtherActor :type "Actor Object Reference") (OtherComp :type "PrimitiveComponent Object Reference") (OtherBodyIndex :type Integer) (bFromSweep :type Boolean) (SweepResult :type "HitResult Structure (by ref)"))
  (if (== OtherActor (`self.SmogRef`))
    (set `self.Dead` true)
    (`/Game/VerticalPlatformer/Cinematics/BP_StartingChar.OnFlowerDied` (`self.PlayerRef`) true)
    (`PaperFlipbookComponent.SetFlipbook` (`self.PaperFlipbook`) "/Game/VerticalPlatformer/Assets/Level/FB_Flower.FB_Flower")))

(fn `UserConstructionScript`)